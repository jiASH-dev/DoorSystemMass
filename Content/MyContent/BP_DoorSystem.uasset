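; BP_DoorSystem is a door actor that swings open and closed on its OpenDoor and CloseDoor events.
; Each event stops the opposing timeline, plays its own from the start, and passes the alpha to a function that sets the door's Z angle.
; When a Pawn leaves the EntryLimiter component's overlap, CanHitted is set to true.
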(event OnComponentEndOverlap(EntryLimiter)
  (params (OverlappedComponent :type Primitive%20Component%20Object%20Reference) (OtherActor :type Actor%20Object%20Reference) (OtherComp :type Primitive%20Component%20Object%20Reference) (OtherBodyIndex :type Integer))
  (Utilities|Casting|CastToPawn OtherActor)
  (Class|DoorSystem|SetCanHitted true))

(event Custom|OpenDoor
  (Audio|Components|Audio|Stop (Variables|Default|GetDoCloseDoor))
  (bind _alpha (Timeline|DoOpenDoor PlayFromStart)
    (:Update
      (Class|DoorSystem|SetDoorZAnglebyAlphatoOpen _alpha))))

(event Custom|CloseDoor
  (Audio|Components|Audio|Stop (Variables|Default|GetDoOpenDoor))
  (bind _alpha (Timeline|DoCloseDoor PlayFromStart)
    (:Update
      (Class|DoorSystem|SetDoorZAnglebyAlphatoClose _alpha))))

(event EventBeginPlay)

(event Collision|EventActorBeginOverlap
  (params (OtherActor :type Actor%20Object%20Reference)))

(event EventTick
  (params (DeltaSeconds :type Float%20%28single-precision%29)))

(fn ConstructionScript)