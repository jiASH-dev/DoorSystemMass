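; BP_MyTriggerBox is a weight-activated trigger volume that opens and closes a door.
; On begin and end overlap, it totals the mass of overlapping components that simulate physics.
; Reaching a fixed mass threshold opens a closed door through DoorSystem, and an end overlap that leaves less than that closes it again.
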(event OnComponentEndOverlap(CollisionComponent)
  (params (OverlappedComponent :type Primitive%20Component%20Object%20Reference) (OtherActor :type Actor%20Object%20Reference) (OtherComp :type Primitive%20Component%20Object%20Reference) (OtherBodyIndex :type Integer))
  (if (not (Class|DoorSystem|GetIsDoorClosed (Variables|Default|GetDoorSystem)))
    (bind _totalmassinvolume (CallFunction|CalculateTotalMassinVolume))
    (if (< _totalmassinvolume 5e+01)
      (Class|DoorSystem|SetIsDoorClosed (Variables|Default|GetDoorSystem) true)
      (Default|CloseDoor (Variables|Default|GetDoorSystem)))))

(event OnComponentBeginOverlap(CollisionComponent)
  (params (OverlappedComponent :type Primitive%20Component%20Object%20Reference) (OtherActor :type Actor%20Object%20Reference) (OtherComp :type Primitive%20Component%20Object%20Reference) (OtherBodyIndex :type Integer) (bFromSweep :type Boolean) (SweepResult :type Hit%20Result%20Structure%20%28by%20ref%29))
  (if (Class|DoorSystem|GetIsDoorClosed (Variables|Default|GetDoorSystem))
    (bind _totalmassinvolume (CallFunction|CalculateTotalMassinVolume))
    (if (>= _totalmassinvolume 5e+01)
      (Class|DoorSystem|SetIsDoorClosed (Variables|Default|GetDoorSystem) false)
      (Default|OpenDoor (Variables|Default|GetDoorSystem)))))

(fn ConstructionScript)

(fn CalculateTotalMassinVolume
  (for _array_element (Class|Actor|GetOverlappingComponents)
    (if (Physics|IsSimulatingPhysics _array_element "None")
      (LocalVariables|SetTotalMass (+ (LocalVariables|GetTotalMass) (Physics|GetMass _array_element)))))
  (return (LocalVariables|GetTotalMass)))